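; Spline-driven track builder for the self-driving car project that generates a road lined with fences on both sides.
; The construction script splits the spline into SegmentLength pieces, adding three laterally offset spline meshes per piece from TrackMesh and FenceMesh.
; Each piece follows the spline's positions and tangents, with tangents clamped to segment length.
; All pieces have query and physics collision, and fences use a custom object channel that distinguishes them from the track.
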(fn `UserConstructionScript`
  (bind _spline (`self.Spline`))
  (bind _spline_2 (`self.Spline`))
  (for _index (range (+ (`KismetMathLibrary.FTrunc` (/ (`SplineComponent.GetSplineLength` (`self.Spline`)) (`self.SegmentLength`))) 1))
    (`|ExecutionSequence`
      (:`then_0`
        (bind _returnvalue (`AddComponent|NODE_AddSplineMeshComponent-0` :`RelativeTransform` (`KismetMathLibrary.MakeTransform` (0.0 500.0 0.0))))
        (`StaticMeshComponent.SetStaticMesh` _returnvalue (`self.TrackMesh`)))
      (:`then_1`
        (bind _returnvalue_2 (`AddComponent|NODE_AddSplineMeshComponent-1` :`RelativeTransform` (`KismetMathLibrary.MakeTransform` (0.0 450.0 0.0))))
        (`StaticMeshComponent.SetStaticMesh` _returnvalue_2 (`self.FenceMesh`)))
      (:`then_2`
        (bind _returnvalue_3 (`AddComponent|NODE_AddSplineMeshComponent-2` :`RelativeTransform` (`KismetMathLibrary.MakeTransform` (0.0 -550.0 0.0))))
        (`StaticMeshComponent.SetStaticMesh` _returnvalue_3 (`self.FenceMesh`)))
      (:`then_3`
        (`SplineMeshComponent.SetForwardAxis` _returnvalue "X" true)
        (`SplineMeshComponent.SetForwardAxis` _returnvalue_2 "X" true)
        (`SplineMeshComponent.SetForwardAxis` _returnvalue_3 "X" true)
        (bind _returnvalue_4 (* _index (`self.SegmentLength`)))
        (bind _returnvalue_5 (* (+ _index 1) (`self.SegmentLength`)))
        (`SplineMeshComponent.SetStartAndEnd` _returnvalue (`SplineComponent.GetLocationAtDistanceAlongSpline` _spline_2 _returnvalue_4 "Local") (`KismetMathLibrary.ClampVectorSize` (`SplineComponent.GetTangentAtDistanceAlongSpline` _spline_2 _returnvalue_4 "Local") 0.0 (`self.SegmentLength`)) (`SplineComponent.GetLocationAtDistanceAlongSpline` _spline _returnvalue_5 "Local") (`KismetMathLibrary.ClampVectorSize` (`SplineComponent.GetTangentAtDistanceAlongSpline` _spline _returnvalue_5 "Local") 0.0 (`self.SegmentLength`)) true)
        (`SplineMeshComponent.SetStartAndEnd` _returnvalue_2 (`SplineComponent.GetLocationAtDistanceAlongSpline` _spline_2 _returnvalue_4 "Local") (`KismetMathLibrary.ClampVectorSize` (`SplineComponent.GetTangentAtDistanceAlongSpline` _spline_2 _returnvalue_4 "Local") 0.0 (`self.SegmentLength`)) (`SplineComponent.GetLocationAtDistanceAlongSpline` _spline _returnvalue_5 "Local") (`KismetMathLibrary.ClampVectorSize` (`SplineComponent.GetTangentAtDistanceAlongSpline` _spline _returnvalue_5 "Local") 0.0 (`self.SegmentLength`)) true)
        (`SplineMeshComponent.SetStartAndEnd` _returnvalue_3 (`SplineComponent.GetLocationAtDistanceAlongSpline` _spline_2 _returnvalue_4 "Local") (`KismetMathLibrary.ClampVectorSize` (`SplineComponent.GetTangentAtDistanceAlongSpline` _spline_2 _returnvalue_4 "Local") 0.0 (`self.SegmentLength`)) (`SplineComponent.GetLocationAtDistanceAlongSpline` _spline _returnvalue_5 "Local") (`KismetMathLibrary.ClampVectorSize` (`SplineComponent.GetTangentAtDistanceAlongSpline` _spline _returnvalue_5 "Local") 0.0 (`self.SegmentLength`)) true)
        (`PrimitiveComponent.SetCollisionEnabled` _returnvalue "QueryAndPhysics")
        (`PrimitiveComponent.SetCollisionEnabled` _returnvalue_2 "QueryAndPhysics")
        (`PrimitiveComponent.SetCollisionEnabled` _returnvalue_3 "QueryAndPhysics")
        (`PrimitiveComponent.SetCollisionObjectType` _returnvalue_2 "ECC_GameTraceChannel1")
        (`PrimitiveComponent.SetCollisionObjectType` _returnvalue_3 "ECC_GameTraceChannel1")))))